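; Game mode that streams a Live Link transform, intended as left-hand tracking, to a local socket server through a raw connection opened on BeginPlay.
; Tick sends time and transform through EncodeTXData and applies the transform to itself; extra SteamVR controller evaluations are discarded.
; The encode and time helpers contain only unconnected nodes (byte packing with axis swap and metre scaling, Unix timestamp).
; Received bytes are ignored, and the HandL-tagged tracker is only printed.
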(event `self.ReceiveBeginPlay`
  (bind _outactors (`GameplayStatics.GetAllActorsOfClassWithTag` "/Game/Blueprints/BP_Tracker.BP_Tracker_C" "HandL"))
  (`KismetSystemLibrary.PrintString` (`KismetSystemLibrary.GetDisplayName` (`|GetArrayItem` _outactors)))
  (bind _returnvalue (`LowEntrySocketConnectionLibrary.RawConnection_CreateCustomBufferSize` "127.0.0.1" 8000 64 (delegate `onConnect`) (delegate `onDisconnect`) (delegate `onRxBytes`)))
  (`KismetSystemLibrary.PrintString` "Connecting...")
  (`LowEntryRawSocketConnection.Connect` _returnvalue))

(event `onConnect`
  (params (SocketConnection :type "LowEntryRawSocketConnection Object Reference"))
  (`KismetSystemLibrary.PrintString` "Connected: ")
  (`LowEntryRawSocketConnection.SendMessage` (stale `self.ReceiveBeginPlay` _returnvalue) (`self.encodeTXData` (`self.getTime`) (`KismetMathLibrary.MakeTransform` (0.0 0.0 0.0)))))

(event `onDisconnect`
  (params (SocketConnection :type "LowEntryRawSocketConnection Object Reference")))

(event `onRxBytes`
  (params (SocketConnection :type "LowEntryRawSocketConnection Object Reference") (Bytes :type "Array of Byte (by ref)")))

(event `self.ReceiveTick`
  (params (DeltaSeconds :type "Float (single-precision)"))
  (bind _transform (`self.evaluateFrame` (make `LiveLinkSubjectName` "SteamVRController_LHR-F7AF3D44")))
  (`self.evaluateFrame` (make `LiveLinkSubjectName` "SteamVRController_LHR-F7AF3D44"))
  (`self.evaluateFrame` (make `LiveLinkSubjectName` "SteamVRController_LHR-F7AF3D44"))
  (`self.evaluateFrame` (make `LiveLinkSubjectName` "SteamVRController_LHR-F7AF3D44"))
  (`self.evaluateFrame` (make `LiveLinkSubjectName` "SteamVRController_LHR-F7AF3D44"))
  (`LowEntryRawSocketConnection.SendMessage` (stale `self.ReceiveBeginPlay` _returnvalue) (`self.encodeTXData` (`self.getTime`) _transform))
  (`self.K2_SetActorTransform` _transform))

(fn `evaluateFrame`
  (params (name :type "LiveLinkSubjectName Structure"))
  (returns (transform :type "Transform Structure"))
  (bind _dataresult (`|EvaluateLiveLinkFrameWithSpecificRole` name "/Script/LiveLinkInterface.LiveLinkTransformRole")
    (:`then`
      _)
    (:`InvalidFrame`
      _))
  (return (break `LiveLinkTransformFrameData` (`.FrameData` (break `LiveLinkTransformBlueprintData` _dataresult)))))

(fn `UserConstructionScript`)